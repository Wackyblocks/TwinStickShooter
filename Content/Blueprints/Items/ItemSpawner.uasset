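; Item spawner actor that drops a random ItemBurst or ItemHealth pickup at a random point inside its SpawnVolume box.
; SpawnItem only spawns while fewer than five ItemHealth actors exist in the level, so ItemBurst count is not capped directly.
; ItemHealth skips spawning when colliding, while ItemBurst leaves collision handling undefined.
; Nothing in this Blueprint calls SpawnItem.
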(event Custom|SpawnItem
  (bind _spawnvolume (Variables|Default|GetSpawnVolume))
  (bind _returnvalue (Components|Box|GetScaledBoxExtent _spawnvolume))
  (bind _returnvalue_2 (Transformation|GetWorldLocation _spawnvolume))
  (bind _returnvalue_3 (Math|Random|RandomPointinBoundingBox _returnvalue_2 _returnvalue))
  (bind _returnvalue_4 (Math|Conversions|ToTransform(Vector) _returnvalue_3))
  ;[1 1 1] Check spawn limit
  (bind _outactors (Actor|GetAllActorsOfClass "/Game/Blueprints/Items/ItemHealth.ItemHealth_C"))
  (if (< (Utilities|Array|Length _outactors) 5)
    ;[1 1 1] Randomizer
    (Variables|Default|SetItemType (Math|Random|RandomIntegerinRange 0 1))
    (if (== (Variables|Default|GetItemType) 0)
      ;[1 1 1] Spawn items
      (Game|SpawnActorfromClass "/Game/Blueprints/Items/ItemBurst.ItemBurst_C" _returnvalue_4 "Undefined" "MultiplyWithRoot" 0 0)
      (else
        (Game|SpawnActorfromClass "/Game/Blueprints/Items/ItemHealth.ItemHealth_C" _returnvalue_4 "DontSpawnIfColliding" "MultiplyWithRoot" 0 0)))))

(event EventBeginPlay)

(event Collision|EventActorBeginOverlap
  (params (OtherActor :type Actor%20Object%20Reference)))

(event EventTick
  (params (DeltaSeconds :type Float%20%28single-precision%29)))

(fn ConstructionScript)