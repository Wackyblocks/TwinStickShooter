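; ItemBurst is a pickup item that grants bursts to the player's hero.
; When its Cube component begins overlapping a HeroCharacter, it plays a pickup sound at its location, sets the hero's Bursts count to a fixed amount rather than adding to it, and destroys itself.
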(event OnComponentBeginOverlap(Cube)
  (params (OverlappedComponent :type Primitive%20Component%20Object%20Reference) (OtherActor :type Actor%20Object%20Reference) (OtherComp :type Primitive%20Component%20Object%20Reference) (OtherBodyIndex :type Integer) (bFromSweep :type Boolean) (SweepResult :type Hit%20Result%20Structure%20%28by%20ref%29))
  ;[1 1 1] Pickup item
  (bind _ashero_character (Utilities|Casting|CastToHeroCharacter OtherActor))
  (Audio|PlaySoundatLocation "/Game/StarterContent/Audio/Shooter/Pickup_item.Pickup_item" (Transformation|GetActorLocation) "0, 0, 0" 1.0 1.0 0.0 0 0 0 0)
  (Variables|/Game/Blueprints/HeroCharacter.HeroCharacter_C|SetBursts _ashero_character 5)
  (Actor|DestroyActor))

(event EventBeginPlay
  (|CallParentFunction) ; This node is disabled and will not be called.\nDrag off pins to build functionality.
)

(event Collision|EventActorBeginOverlap
  (params (OtherActor :type Actor%20Object%20Reference))
  (|CallParentFunction OtherActor) ; This node is disabled and will not be called.\nDrag off pins to build functionality.
)

(event EventTick
  (params (DeltaSeconds :type Float%20%28single-precision%29))
  (|CallParentFunction DeltaSeconds) ; This node is disabled and will not be called.\nDrag off pins to build functionality.
)

(fn ConstructionScript
  (|CallParentFunction))