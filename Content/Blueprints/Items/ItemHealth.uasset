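; Health pickup item that a HeroCharacter collects by touching it.
; On BeginPlay it snaps to the first Visibility hit of a line trace, whose end is a fixed world point deep below the origin rather than directly beneath the item.
; Cube overlap by the hero plays a sound, applies AddHealth through AffectHealth and destroys the item.
; A DeleteItems event also destroys it and prints a confirmation.
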(event OnComponentBeginOverlap(Cube)
  (params (OverlappedComponent :type Primitive%20Component%20Object%20Reference) (OtherActor :type Actor%20Object%20Reference) (OtherComp :type Primitive%20Component%20Object%20Reference) (OtherBodyIndex :type Integer) (bFromSweep :type Boolean) (SweepResult :type Hit%20Result%20Structure%20%28by%20ref%29))
  ;[1 1 1] Pickup item
  (bind _ashero_character (Utilities|Casting|CastToHeroCharacter OtherActor))
  (Audio|PlaySoundatLocation "/Game/StarterContent/Audio/Shooter/Pickup_item.Pickup_item" (Transformation|GetActorLocation) "0, 0, 0" 1.0 1.0 0.0 0 0 0 0)
  (Default|AffectHealth _ashero_character (Variables|Default|GetAddHealth))
  (Actor|DestroyActor))

(event Custom|DeleteItems
  (Actor|DestroyActor)
  (Development|PrintText "Items deleted"))

(event EventBeginPlay
  ;[1 1 1] Snap item to ground
  (bind _outhit (Collision|LineTraceByChannel (Transformation|GetActorLocation) "0.000000,0.000000,-10000.000000" "TraceTypeQuery1" false 0 "None"))
  (if (.bBlockingHit (Collision|BreakHitResult _outhit))
    (Transformation|SetActorLocation (.ImpactPoint (Collision|BreakHitResult _outhit)) false false)))

(event Collision|EventActorBeginOverlap
  (params (OtherActor :type Actor%20Object%20Reference)))

(event EventTick
  (params (DeltaSeconds :type Float%20%28single-precision%29)))

(fn ConstructionScript)